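; Player controller that drives a BP_CharacterBase pawn with camera-relative movement, look, jump and melee attack.
; On BeginPlay it caches the pawn and creates the WBP_HUD widget, which receives new abilities through AddAbilitytoUI.
; Five slot inputs read the ability class from the matching HUD slot and activate it by class on the character's Ability System Component, so the HUD serves as the loadout source.
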(event EventAddAbilitytoUI
  (params (AbilityToAdd :type Gameplay%20Ability%20Info%20Structure))
  (Default|AddAbilitytoSlots (Variables|Default|GetHUDRef) AbilityToAdd))

(event EventBeginPlay
  (bind _asbp_character_base (Utilities|Casting|CastToBP_CharacterBase (Pawn|GetControlledPawn))
    (:then
      (Variables|Default|SetControlledCharacter _asbp_character_base))
    (:CastFailed
      (Development|PrintString "Failed to cast ControlledPawn to Character!" true true "(R=1.000000,G=0.000000,B=0.000000,A=1.000000)")))
  (bind _returnvalue (UserInterface|CreateWidget "/Game/UI/WBP_HUD.WBP_HUD_C"))
  (bind _output_get (Variables|Default|SetHUDRef _returnvalue))
  (UserInterface|Viewport|AddtoViewport _output_get 0))

(event Input|ActionEvents|InputActionJump
  (params (Key :type Key%20Structure :default "None"))
  (bind _controlledcharacter (Variables|Default|GetControlledCharacter))
  ;[1 1 1] Basic Controls
  (:Pressed
    (Utilities|IsValid _controlledcharacter
      (:Is%20Valid
        (Character|Jump _controlledcharacter)))))

(event Input|ActionEvents|InputActionPrimaryAttack
  (params (Key :type Key%20Structure :default "None"))
  (bind _controlledcharacter (Variables|Default|GetControlledCharacter))
  ;[1 1 1] Ability Controls
  (:Pressed
    (Utilities|IsValid _controlledcharacter
      (:Is%20Valid
        (Default|MeleeAttack _controlledcharacter)))))

(event Input|ActionEvents|InputActionSlotOneAbility
  (params (Key :type Key%20Structure :default "None"))
  ;[1 1 1] Ability Controls
  (:Pressed
    (CallFunction|TryActivateAbilityinSlot)))

(event Input|ActionEvents|InputActionSlotTwoAbility
  (params (Key :type Key%20Structure :default "None"))
  ;[1 1 1] Ability Controls
  (:Pressed
    (CallFunction|TryActivateAbilityinSlot 1)))

(event Input|ActionEvents|InputActionSlotThreeAbility
  (params (Key :type Key%20Structure :default "None"))
  ;[1 1 1] Ability Controls
  (:Pressed
    (CallFunction|TryActivateAbilityinSlot 2)))

(event Input|ActionEvents|InputActionSlotFourAbility
  (params (Key :type Key%20Structure :default "None"))
  ;[1 1 1] Ability Controls
  (:Pressed
    (CallFunction|TryActivateAbilityinSlot 3)))

(event Input|ActionEvents|InputActionSlotFiveAbility
  (params (Key :type Key%20Structure :default "None"))
  ;[1 1 1] Ability Controls
  (:Pressed
    (CallFunction|TryActivateAbilityinSlot 4)))

(event Input|AxisEvents|InputAxisMoveForward
  (params (AxisValue :type Float%20%28single-precision%29))
  (bind _controlledcharacter (Variables|Default|GetControlledCharacter))
  ;[1 1 1] Basic Controls
  (Utilities|IsValid _controlledcharacter
    (:Is%20Valid
      (Pawn|Input|AddMovementInput _controlledcharacter (Math|Vector|GetForwardVector (Camera|GetCameraRotation (Game|GetPlayerCameraManager 0))) AxisValue false))))

(event Input|AxisEvents|InputAxisMoveRight
  (params (AxisValue :type Float%20%28single-precision%29))
  (bind _controlledcharacter (Variables|Default|GetControlledCharacter))
  ;[1 1 1] Basic Controls
  (Utilities|IsValid _controlledcharacter
    (:Is%20Valid
      (Pawn|Input|AddMovementInput _controlledcharacter (Math|Vector|GetRightVector (Camera|GetCameraRotation (Game|GetPlayerCameraManager 0))) AxisValue false))))

(event Input|AxisEvents|InputAxisLookingUp
  (params (AxisValue :type Float%20%28single-precision%29))
  ;[1 1 1] Basic Controls
  (Class|PlayerController|AddPitchInput AxisValue))

(event Input|AxisEvents|InputAxisLookingRight
  (params (AxisValue :type Float%20%28single-precision%29))
  ;[1 1 1] Basic Controls
  (Class|PlayerController|AddYawInput AxisValue))

(fn ConstructionScript)

(fn TryActivateAbilityinSlot
  (params (SlotNumber :type Integer))
  (bind _hudref (Variables|Default|GetHUDRef))
  (bind _controlledcharacter (Variables|Default|GetControlledCharacter))
  (bind (_abilityclass _isvalid) (Default|GetSlotAbilityClass _hudref SlotNumber))
  (if (and _isvalid (Utilities|IsValid _controlledcharacter))
    (Abilities|TryActivateAbilitybyClass (Ability|GetAbilitySystemComponent _controlledcharacter) _abilityclass true)))