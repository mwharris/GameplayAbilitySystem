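; BP_PlayerCharacter is the player character Blueprint that relays health and mana changes to the HUD.
; On BeginPlay it casts its controller to BP_PlayerController and caches it.
; The health and mana change events use that controller's HUDRef to set each glass ball's percentage from current over max.
; The mana event also prints the current value to screen.
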(event EventBeginPlay
  (|CallParentFunction)
  (bind _asbp_player_controller (Utilities|Casting|CastToBP_PlayerController (Pawn|GetController)))
  (Variables|Default|SetPlayerController _asbp_player_controller))

(event EventOnManaChanged
  (params (Mana :type Float%20%28single-precision%29) (MaxMana :type Float%20%28single-precision%29))
  (bind _playercontroller (Variables|Default|GetPlayerController))
  (Utilities|IsValid _playercontroller
    (:Is%20Valid
      (Development|PrintString (Utilities|String|ToString(Float) Mana))
      (Default|SetPercentage (Variables|/Game/UI/WBP_HUD.WBP_HUD_C|GetManaGlassBall (Variables|/Game/Blueprints/BP_PlayerController.BP_PlayerController_C|GetHUDRef _playercontroller)) (/ Mana MaxMana)))))

(event EventOnHealthChanged
  (params (Health :type Float%20%28single-precision%29) (MaxHealth :type Float%20%28single-precision%29))
  (bind _playercontroller (Variables|Default|GetPlayerController))
  (Utilities|IsValid _playercontroller
    (:Is%20Valid
      (Default|SetPercentage (Variables|/Game/UI/WBP_HUD.WBP_HUD_C|GetHealthGlassBall (Variables|/Game/Blueprints/BP_PlayerController.BP_PlayerController_C|GetHUDRef _playercontroller)) (/ Health MaxHealth)))))

(fn ConstructionScript
  (|CallParentFunction))