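; Fire Blast gameplay ability that pulls nearby characters toward the caster, then blasts them away with damage and a stun.
; It commits, starts the UI cooldown and plays a montage whose gameplay events time the pull and push phases.
; The pull event gathers targets with an instant radius target actor and stores them; the push event applies the damage effect and reverses the impulse on that same set.
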(event Ability|EventActivateAbility
  (|CallParentFunction)
  (Ability|CommitAbility)
  (CallFunction|DoUICooldown)
  (|PlayMontageandWaitProxy "None" "/Game/Blueprints/Characters/Animation/AM_Shinbi_FireBlast.AM_Shinbi_FireBlast" 1.0 "None" true 1.0 0.0
    (:then
      (Ability|Tasks|WaitGameplayEvent "(TagName=\"skill.fireBlast.pull\")" 0
        (:EventReceived
          (bind _data (|WaitTargetData :ConfirmationType "Instant" :Class "/Script/AbilitySystem.GATargetActorAround" :Radius 6e+02 :ReticleClass 0)
            (:then
              ;[1 1 1] Push enemies away
              (Ability|Tasks|WaitGameplayEvent "(TagName=\"skill.fireBlast.push\")" 0
                (:EventReceived
                  (GameplayEffects|ApplyGameplayEffectToTarget (Variables|Default|GetTargetDataHandle) "/Game/Blueprints/Characters/GameplayAbilities/FireBlast/GE_FireBlast_Damage.GE_FireBlast_Damage_C" 1 1)
                  (for _array_element (Ability|TargetData|GetActorsfromTargetData (Variables|Default|GetTargetDataHandle))
                    (bind _asbp_character_base (Utilities|Casting|CastToBP_CharacterBase _array_element))
                    (Default|PushCharacter _asbp_character_base (* (CallFunction|GetTargettoPlayerVector _asbp_character_base) -1.0) 2e+03 3.0)))))
            (:ValidData
              ;[1 1 1] Pull enemies closer
              (bind _output_get (Variables|Default|SetTargetDataHandle _data))
              (for _array_element_2 (Ability|TargetData|GetActorsfromTargetData _output_get)
                (bind _asbp_character_base_2 (Utilities|Casting|CastToBP_CharacterBase _array_element_2))
                (Default|PushCharacter _asbp_character_base_2 (CallFunction|GetTargettoPlayerVector _asbp_character_base_2) 1e+03 3.0)))
            (:Cancelled
              (Ability|EndAbility))))))
    (:OnCompleted
      (Ability|EndAbility :!label _label))
    (:OnBlendOut
      (goto _label))
    (:OnInterrupted
      (goto _label))
    (:OnCancelled
      (goto _label))))

(fn GetTargettoPlayerVector
  (params (self2 :type Actor%20Object%20Reference))
  (return (Math|Vector|Normalize (- (Transformation|GetActorLocation (Ability|GetOwningActorfromActorInfo)) (Transformation|GetActorLocation self2)))))