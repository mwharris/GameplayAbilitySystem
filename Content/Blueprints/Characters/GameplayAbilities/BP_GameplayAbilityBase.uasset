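; Base Gameplay Ability Blueprint that supplies shared owner caching, cost checking and cooldown UI helpers for character abilities.
; On activation it caches the owning BP_CharacterBase and its BP_PlayerController.
; GetAbilityInfo drives both the affordability check against the character's Health, Mana or Strength attribute and the search for the matching HUD slot to start its cooldown display.
; A helper also returns the normalized direction from the character to a target actor.
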(event Ability|EventActivateAbility
  (CallFunction|SetPlayerInfo))

(fn SetPlayerInfo
  (Utilities|FlowControl|Sequence
    (:then_0
      (Utilities|IsValid (Variables|Default|GetBPCharacterBaseRef)
        (:Is%20Not%20Valid
          (bind _asbp_character_base (Utilities|Casting|CastToBP_CharacterBase (Ability|GetOwningActorfromActorInfo)))
          (Variables|Default|SetBPCharacterBaseRef _asbp_character_base))))
    (:then_1
      (Utilities|IsValid (Variables|Default|GetBPCharacterBaseRef)
        (:Is%20Valid
          (Utilities|IsValid (Variables|Default|GetBPPlayerControllerRef)
            (:Is%20Not%20Valid
              (bind _asbp_player_controller (Utilities|Casting|CastToBP_PlayerController (Pawn|GetController (Variables|Default|GetBPCharacterBaseRef))))
              (Variables|Default|SetBPPlayerControllerRef _asbp_player_controller))))))))

(fn GetDirectiontoTarget
  (params (TargetActor :type Actor%20Object%20Reference))
  (return (Math|Vector|Normalize (- (Transformation|GetActorLocation TargetActor) (Transformation|GetActorLocation (Variables|Default|GetBPCharacterBaseRef))))))

(fn DoUICooldown
  (bind _bpplayercontrollerref (Variables|Default|GetBPPlayerControllerRef))
  (Utilities|IsValid _bpplayercontrollerref
    (:Is%20Valid
      (for _array_element (Variables|/Game/UI/WBP_HUD.WBP_HUD_C|GetSlots (Variables|/Game/Blueprints/BP_PlayerController.BP_PlayerController_C|GetHUDRef _bpplayercontrollerref))
        (bind _returnvalue (Class|GameplayAbilityBase|GetAbilityInfo))
        (if (== (.abilityclass _returnvalue) (.abilityclass (Variables|/Game/UI/WBP_Ability_Slot.WBP_Ability_Slot_C|GetAbility%20Info _array_element)))
          (Default|StartCooldown _array_element)
          (return))))))

(fn IsAbilityCostAvailable
  (bind _returnvalue (Class|GameplayAbilityBase|GetAbilityInfo))
  (LocalVariables|SetCost (Math|Float|Absolute(Float) (.cost _returnvalue)))
  (switch Utilities|FlowControl|Switch|SwitchonEAbilityCostType (.costtype _returnvalue)
    (:Health
      (if (>= (.currentvalue (Variables|/Script/AbilitySystem.AttributeSetBase|GetHealth (Variables|/Script/AbilitySystem.CharacterBase|GetAttributeSetComp (Variables|Default|GetBPCharacterBaseRef)))) (LocalVariables|GetCost))
        (return true)
        (else
          (return false))))
    (:Mana
      (if (>= (.currentvalue (Variables|/Script/AbilitySystem.AttributeSetBase|GetMana (Variables|/Script/AbilitySystem.CharacterBase|GetAttributeSetComp (Variables|Default|GetBPCharacterBaseRef)))) (LocalVariables|GetCost))
        (return true)
        (else
          (return false))))
    (:Strength
      (if (>= (.currentvalue (Variables|/Script/AbilitySystem.AttributeSetBase|GetStrength (Variables|/Script/AbilitySystem.CharacterBase|GetAttributeSetComp (Variables|Default|GetBPCharacterBaseRef)))) (LocalVariables|GetCost))
        (return true)
        (else
          (return false))))))