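; GA_GroundBlast is a gameplay ability that lets a Shinbi character pick a ground target, then damages and launches the characters caught there.
; It plays a targeting montage, waits out its length, then awaits user confirmation through BP_GATargetActorGroundSelect.
; On confirmation, the cast montage starts while GE_GroundBlast_Damage and an upward stunning PushCharacter hit the targets immediately.
; The ability ends when that montage finishes or is interrupted, or targeting is cancelled.
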(event Ability|EventActivateAbility
  (|CallParentFunction)
  (|PlayMontageandWaitProxy "None" "/Game/Blueprints/Characters/Animation/AM_Shinbi_GroundBlast_Targeting.AM_Shinbi_GroundBlast_Targeting" 1.0 "None" true 1.0 0.0
    (:then
      (Utilities|FlowControl|Delay (Variables|/Script/Engine.AnimSequenceBase|GetSequenceLength (Animation|GetCurrentMontage :!class /Script/GameplayAbilities.GameplayAbility)))
      (bind _data (|WaitTargetData :ConfirmationType "UserConfirmed" :Class "/Game/Blueprints/Characters/GameplayAbilities/GroundBlast/BP_GATargetActorGroundSelect.BP_GATargetActorGroundSelect_C" :ReticleClass 0)
        (:ValidData
          (|PlayMontageandWaitProxy "None" "/Game/Blueprints/Characters/Animation/AM_Shinbi_GroundBlast_Cast.AM_Shinbi_GroundBlast_Cast" 1.0 "None" true 1.0 0.0
            (:then
              (GameplayEffects|ApplyGameplayEffectToTarget _data "/Game/Blueprints/Characters/GameplayAbilities/GroundBlast/GE_GroundBlast_Damage.GE_GroundBlast_Damage_C" 1 1)
              (for _array_element (Ability|TargetData|GetActorsfromTargetData _data)
                (bind _asbp_character_base (Utilities|Casting|CastToBP_CharacterBase _array_element))
                (Default|PushCharacter _asbp_character_base "0, 0,1.000000" 5e+02 2.0)))
            (:OnCompleted
              (Ability|EndAbility :!label _label))
            (:OnBlendOut
              (goto _label))
            (:OnInterrupted
              (goto _label))
            (:OnCancelled
              (goto _label))))
        (:Cancelled
          (goto _label))))))