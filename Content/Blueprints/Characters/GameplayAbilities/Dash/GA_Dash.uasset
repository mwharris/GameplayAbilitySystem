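; Dash gameplay ability that launches the character forward and damages, pushes and stuns targets it hits.
; On activation it commits, zeroes ground friction, sets pawn collision to overlap, applies a forward impulse and plays the Shinbi dash montage.
; While dashing, it waits for a dealDamage gameplay event to apply the damage effect and push.
; When the montage ends or is interrupted, it restores friction and collision and ends.
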(event Ability|EventActivateAbility
  (bind _bpcharacterbaseref (Variables|Default|GetBPCharacterBaseRef))
  (|CallParentFunction)
  (Ability|CommitAbility)
  (Utilities|IsValid (Variables|Default|GetBPCharacterBaseRef)
    (:Is%20Valid
      (CallFunction|PreDashSetup)
      ;[1 1 1] Add a Dash impulse to push our character
      (Physics|AddImpulse (Variables|/Script/Engine.Character|GetCharacterMovement _bpcharacterbaseref) (* (Transformation|GetActorForwardVector _bpcharacterbaseref) 2e+03) true)
      ;[1 1 1] Play Dash animation
      (|PlayMontageandWaitProxy "None" "/Game/Blueprints/Characters/Animation/AM_Shinbi_Dash.AM_Shinbi_Dash" 1.0 "None" true 1.0 0.0
        (:then
          ;[1 1 1] Apply Gameplay Effect if we receive a dealDamage Gameplay Event
          (bind _payload (Ability|Tasks|WaitGameplayEvent "(TagName=\"skill.dash.dealDamage\")" 0)
            (:EventReceived
              (GameplayEffects|ApplyGameplayEffectToTarget (Ability|TargetData|AbilityTargetDatafromActor (.Target (Utilities|Struct|BreakGameplayEventData _payload))) "/Game/Blueprints/Characters/GameplayAbilities/Dash/GE_Dash_Damage.GE_Dash_Damage_C" 1 1)
              (bind _asbp_character_base (Utilities|Casting|CastToBP_CharacterBase (.Target (Utilities|Struct|BreakGameplayEventData _payload))))
              (Default|PushCharacter _asbp_character_base (CallFunction|GetDirectiontoTarget _asbp_character_base) 4e+03 5.0))))
        (:OnCompleted
          ;[1 1 1] EndAbility on animation finished
          (CallFunction|PostDashSetup :!label _label)
          (Ability|EndAbility))
        (:OnBlendOut
          (goto _label))
        (:OnInterrupted
          (goto _label))
        (:OnCancelled
          (goto _label))))
    (:Is%20Not%20Valid
      (Ability|EndAbility))))

(fn PreDashSetup
  (bind _bpcharacterbaseref (Variables|Default|GetBPCharacterBaseRef))
  (bind _bpcharacterbaseref_2 (Variables|Default|GetBPCharacterBaseRef))
  (bind _charactermovement (Variables|/Script/Engine.Character|GetCharacterMovement _bpcharacterbaseref))
  (Utilities|FlowControl|Sequence
    (:then_0
      (Utilities|IsValid _bpcharacterbaseref
        (:Is%20Valid
          (Variables|Default|SetOriginal%20Ground%20Friction (Variables|/Script/Engine.CharacterMovementComponent|GetGroundFriction _charactermovement))
          (Variables|/Script/Engine.CharacterMovementComponent|SetGroundFriction _charactermovement 0.0))))
    (:then_1
      (Utilities|IsValid _bpcharacterbaseref_2
        (:Is%20Valid
          (Default|SetCollisionResponsetoPawn _bpcharacterbaseref_2 "ECR_Overlap"))))))

(fn PostDashSetup
  (bind _bpcharacterbaseref (Variables|Default|GetBPCharacterBaseRef))
  (bind _bpcharacterbaseref_2 (Variables|Default|GetBPCharacterBaseRef))
  (Utilities|FlowControl|Sequence
    (:then_0
      (Utilities|IsValid _bpcharacterbaseref
        (:Is%20Valid
          (Variables|/Script/Engine.CharacterMovementComponent|SetGroundFriction (Variables|/Script/Engine.Character|GetCharacterMovement _bpcharacterbaseref) (Variables|Default|GetOriginal%20Ground%20Friction)))))
    (:then_1
      (Utilities|IsValid _bpcharacterbaseref_2
        (:Is%20Valid
          (Default|SetCollisionResponsetoPawn _bpcharacterbaseref_2 "ECR_Block"))))))