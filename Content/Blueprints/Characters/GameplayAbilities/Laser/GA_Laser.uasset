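; Gameplay ability for a channeled laser: plays a cast montage and attaches a BP_Laser to the character's mesh socket after a short delay.
; The camera controls character rotation while active, and each damage event checks mana, then damages, pushes and briefly stuns targets away from the laser's end.
; Insufficient mana or montage end stops the ability, removing the mana-drain effect, destroying the laser and restoring rotation.
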(event Ability|EventActivateAbility
  (bind _bpcharacterbaseref (Variables|Default|GetBPCharacterBaseRef))
  (|CallParentFunction)
  (Ability|CommitAbility)
  (CallFunction|DoUICooldown)
  (|PlayMontageandWaitProxy "None" "/Game/Blueprints/Characters/Animation/AM_Shinbi_Cast_Laser.AM_Shinbi_Cast_Laser" 1.0 "None" true 1.0 0.0
    (:then
      (Utilities|FlowControl|Delay 0.4)
      (bind _spawnedactor (|SpawnActor :Class "/Game/Blueprints/Characters/GameplayAbilities/Laser/BP_Laser.BP_Laser_C" :Instigator _bpcharacterbaseref)
        (:then
          (bind _output_get (Variables|Default|SetLaserActor _spawnedactor))
          (Transformation|AttachComponentToComponent _output_get (Variables|/Script/Engine.Character|GetMesh _bpcharacterbaseref) "LaserSocket" "SnapToTarget" "SnapToTarget" "KeepRelative" true)
          (Default|MakeCameraControlRotation (Variables|Default|GetBPCharacterBaseRef) true)
          (bind _payload (Ability|Tasks|WaitGameplayEvent "(TagName=\"skill.laser.dealDamage\")" 0)
            (:EventReceived
              (bind _result (CallFunction|IsManaCostAvailable))
              (if _result
                (GameplayEffects|ApplyGameplayEffectToTarget (.TargetData (Utilities|Struct|BreakGameplayEventData _payload)) "/Game/Blueprints/Characters/GameplayAbilities/Laser/GE_Laser_Damage.GE_Laser_Damage_C" 1 1)
                (for _array_element (Ability|TargetData|GetActorsfromTargetData (.TargetData (Utilities|Struct|BreakGameplayEventData _payload)))
                  (bind _asbp_character_base (Utilities|Casting|CastToBP_CharacterBase _array_element))
                  (Default|PushCharacter _asbp_character_base (CallFunction|GetLaserPushDirection _asbp_character_base) 5e+02 0.3))
                (else
                  (Ability|EndAbility))))))))
    (:OnCompleted
      (Ability|EndAbility :!label _label))
    (:OnBlendOut
      (goto _label))
    (:OnInterrupted
      (goto _label))
    (:OnCancelled
      (goto _label))))

(event Ability|EventOnEndAbility
  (params (bWasCancelled :type Boolean))
  (Ability|RemoveGameplayEffectFromOwnerWithAssetTags "(GameplayTags=((TagName=\"skill.laser.drainMana\")))")
  (Actor|DestroyActor (Variables|Default|GetLaserActor))
  (Default|MakeCameraControlRotation (Variables|Default|GetBPCharacterBaseRef) false))

(fn GetLaserPushDirection
  (params (CharacterToPush :type Actor%20Object%20Reference))
  (return (Math|Vector|Normalize (- (Transformation|GetActorLocation CharacterToPush) (Transformation|GetWorldLocation (Variables|/Game/Blueprints/Characters/GameplayAbilities/Laser/BP_Laser.BP_Laser_C|GetLaserEndCollider (.AsBP%20Laser (Utilities|Casting|CastToBP_Laser (Variables|Default|GetLaserActor)))))))))