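; Laser beam actor for a gameplay ability that tracks hostile characters at the beam's end and reports them for damage.
; Each tick it feeds the end collider's distance, minus the original beam length, to the AnimBP's end bone offset to stretch the mesh.
; End-collider overlaps maintain a list of characters hostile to the instigator.
; A looping timer sends that list as target data in a deal-damage gameplay event to the instigator.
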(event OnComponentBeginOverlap(LaserEndCollider)
  (params (OverlappedComponent :type Primitive%20Component%20Object%20Reference) (OtherActor :type Actor%20Object%20Reference) (OtherComp :type Primitive%20Component%20Object%20Reference) (OtherBodyIndex :type Integer) (bFromSweep :type Boolean) (SweepResult :type Hit%20Result%20Structure%20%28by%20ref%29))
  ;[1 1 1] Laser hit detection
  (bind _asbp_character_base (Utilities|Casting|CastToBP_CharacterBase OtherActor))
  (bind _asbp_character_base_2 (Utilities|Casting|CastToBP_CharacterBase (Game|GetInstigator)))
  (bind _returnvalue (Class|CharacterBase|IsOtherHostile _asbp_character_base_2 _asbp_character_base))
  (if _returnvalue
    (Utilities|Array|AddUnique (Variables|Default|GetOverlappingActors) _asbp_character_base)))

(event OnComponentEndOverlap(LaserEndCollider)
  (params (OverlappedComponent :type Primitive%20Component%20Object%20Reference) (OtherActor :type Actor%20Object%20Reference) (OtherComp :type Primitive%20Component%20Object%20Reference) (OtherBodyIndex :type Integer))
  ;[1 1 1] Laser hit detection
  (bind _asbp_character_base (Utilities|Casting|CastToBP_CharacterBase OtherActor))
  (Utilities|Array|RemoveItem (Variables|Default|GetOverlappingActors) _asbp_character_base))

(event EventBeginPlay
  (bind _asanim_bp_laser (Utilities|Casting|CastToAnimBP_Laser (Components|SkeletalMesh|GetAnimInstance (Variables|Default|GetLaserMesh))))
  (Variables|Default|SetAnimBPLaser _asanim_bp_laser)
  (Variables|Default|SetBeamOriginalLength (Math|Vector|VectorLength (- (Transformation|GetSocketLocation (Variables|Default|GetLaserMesh) "end") (Transformation|GetActorLocation))))
  (Utilities|Time|SetTimerbyFunctionName self "SendDealDamageEvent" 0.3 true))

(event EventTick
  (params (DeltaSeconds :type Float%20%28single-precision%29))
  (Variables|/Game/Blueprints/Characters/GameplayAbilities/Laser/LaserAssets/AnimBP_Laser.AnimBP_Laser_C|SetEndBoneOffset (Variables|Default|GetAnimBPLaser) (Math|Vector|MakeVector (- (Math|Vector|VectorLength (- (Transformation|GetWorldLocation (Variables|Default|GetLaserEndCollider)) (Transformation|GetActorLocation))) (Variables|Default|GetBeamOriginalLength)) 0.0 0.0)))

(fn ConstructionScript)

(fn SendDealDamageEvent
  (if (> (Utilities|Array|Length (Variables|Default|GetOverlappingActors)) 0)
    _
    (else
      _))
  (Ability|SendGameplayEventtoActor (Game|GetInstigator) "(TagName=\"skill.laser.dealDamage\")" (Utilities|Struct|MakeGameplayEventData "(TagName=\"\")" 0 0 0 0 "()" "(GameplayTags=)" "(GameplayTags=)" 0.0 (Ability|TargetData|AbilityTargetDatafromActorArray (Variables|Default|GetOverlappingActors)))))