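; BP_Enemy is an enemy character Blueprint with a health bar widget and an AI controller.
; On BeginPlay it caches the WBP_HealthBar widget, then the AIC_Enemy controller, which is skipped if the widget cast fails.
; OnHealthChanged sets the bar to the ratio of current to maximum health when the widget reference is valid.
; The controller reference is only stored here, and Tick is disabled.
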(event EventBeginPlay
  (|CallParentFunction)
  (bind _aswbp_health_bar (Utilities|Casting|CastToWBP_HealthBar (UserInterface|GetUserWidgetObject (Variables|Default|GetHealthBar))))
  (Variables|Default|SetHealthBarRef _aswbp_health_bar)
  (bind _asaic_enemy (Utilities|Casting|CastToAIC_Enemy (Pawn|GetController)))
  (Variables|Default|SetAIControllerRef _asaic_enemy))

(event EventTick
  (params (DeltaSeconds :type Float%20%28single-precision%29))
  (|CallParentFunction DeltaSeconds) ; This node is disabled and will not be called.\nDrag off pins to build functionality.
)

(event EventOnHealthChanged
  (params (Health :type Float%20%28single-precision%29) (MaxHealth :type Float%20%28single-precision%29))
  (Utilities|IsValid (Variables|Default|GetHealthBarRef)
    (:Is%20Valid
      (Default|SetPercentage (Variables|Default|GetHealthBarRef) (/ Health MaxHealth)))))

(fn ConstructionScript
  (|CallParentFunction))