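; Base character Blueprint that uses the Gameplay Ability System for melee, health regen and dash abilities.
; It grants the abilities on BeginPlay and activates each by class through its own event.
; Sword and capsule overlaps with hostile characters send damage gameplay events to itself, with an exclusion list preventing repeat dash hits.
; It also handles montage-timed death, knockback with temporarily zeroed friction and optional stun, and pawn collision response changes.
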(event OnComponentBeginOverlap(SwordCollider)
  (params (OverlappedComponent :type Primitive%20Component%20Object%20Reference) (OtherActor :type Actor%20Object%20Reference) (OtherComp :type Primitive%20Component%20Object%20Reference) (OtherBodyIndex :type Integer) (bFromSweep :type Boolean) (SweepResult :type Hit%20Result%20Structure%20%28by%20ref%29))
  ;[1 1 1] Melee Ability
  (bind _asbp_character_base (Utilities|Casting|CastToBP_CharacterBase OtherActor))
  (bind _returnvalue (Class|CharacterBase|IsOtherHostile _asbp_character_base))
  (if (and _returnvalue (!= OtherActor self))
    (Ability|SendGameplayEventtoActor self "(TagName=\"skill.melee.dealDamage\")" (Utilities|Struct|MakeGameplayEventData "(TagName=\"\")" 0 OtherActor))))

(event OnComponentBeginOverlap(CapsuleComponent)
  (params (OverlappedComponent :type Primitive%20Component%20Object%20Reference) (OtherActor :type Actor%20Object%20Reference) (OtherComp :type Primitive%20Component%20Object%20Reference) (OtherBodyIndex :type Integer) (bFromSweep :type Boolean) (SweepResult :type Hit%20Result%20Structure%20%28by%20ref%29))
  (bind _self self)
  ;[1 1 1] OnComponentBegin Overlap
  (bind _asbp_character_base (Utilities|Casting|CastToBP_CharacterBase OtherActor))
  (bind _returnvalue (Class|CharacterBase|IsOtherHostile _asbp_character_base _self))
  (if _returnvalue
    (if (not (Utilities|Array|ContainsItem (Variables|Default|GetOverlapExcludes) OtherActor))
      (Utilities|Array|AddUnique (Variables|Default|GetOverlapExcludes) OtherActor)
      (Ability|SendGameplayEventtoActor self "(TagName=\"skill.dash.dealDamage\")" (Utilities|Struct|MakeGameplayEventData "(TagName=\"\")" _self OtherActor)))))

(event Custom|MeleeAttack
  ;[1 1 1] Melee Ability
  (Abilities|TryActivateAbilitybyClass (Variables|Default|GetAbilitySystemComp) "/Game/Blueprints/Characters/GameplayAbilities/Melee/GA_Melee.GA_Melee_C" true))

(event Custom|HealthRegen
  ;[1 1 1] Health Regen Ability
  (Abilities|TryActivateAbilitybyClass (Variables|Default|GetAbilitySystemComp) "/Game/Blueprints/Characters/GameplayAbilities/HealthRegen/GA_HealthRegen.GA_HealthRegen_C" true))

(event Custom|Dash
  ;[1 1 1] Dash Abililty
  (Abilities|TryActivateAbilitybyClass (Variables|Default|GetAbilitySystemComp) "/Game/Blueprints/Characters/GameplayAbilities/Dash/GA_Dash.GA_Dash_C" true))

(event Custom|PushCharacter
  (params (ImpulseDirection :type Vector) (PushStrength :type Float%20%28single-precision%29) (StunDuration :type Float%20%28single-precision%29))
  (bind _charactermovement (Variables|Character|GetCharacterMovement))
  ;[1 1 1] Character pushed by an effect
  (Variables|Default|SetDefault%20Ground%20Friction (Variables|/Script/Engine.CharacterMovementComponent|GetGroundFriction _charactermovement))
  (Variables|/Script/Engine.CharacterMovementComponent|SetGroundFriction _charactermovement 0.0)
  (Physics|AddImpulse (Variables|Character|GetCharacterMovement) (* ImpulseDirection PushStrength) true)
  (if (> StunDuration 0.0)
    (Class|CharacterBase|HitStun StunDuration))
  (Utilities|FlowControl|Delay 0.3)
  (Variables|/Script/Engine.CharacterMovementComponent|SetGroundFriction (Variables|Character|GetCharacterMovement) (Variables|Default|GetDefault%20Ground%20Friction)))

(event EventBeginPlay
  (Class|CharacterBase|AcquireAblities (Utilities|Array|MakeArray "/Game/Blueprints/Characters/GameplayAbilities/Melee/GA_Melee.GA_Melee_C" "/Game/Blueprints/Characters/GameplayAbilities/HealthRegen/GA_HealthRegen.GA_HealthRegen_C" "/Game/Blueprints/Characters/GameplayAbilities/Dash/GA_Dash.GA_Dash_C")))

(event EventDie
  (bind _returnvalue (Animation|PlayAnimMontage "/Game/Blueprints/Characters/Animation/AM_Shinbi_Die.AM_Shinbi_Die" 1.0 "None"))
  (Utilities|FlowControl|Delay _returnvalue)
  (Actor|DestroyActor))

(fn ConstructionScript)

(fn SetCollisionResponsetoPawn
  (params (NewResponse :type ECollisionResponse%20Enum :default "ECR_Ignore"))
  (Collision|SetCollisionResponsetoChannel (Variables|Default|GetCapsuleComponent) "ECC_Pawn" NewResponse))